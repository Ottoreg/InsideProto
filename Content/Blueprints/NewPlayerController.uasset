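; Player controller that lets the player switch control between three side-scroller characters and a separate Flame actor.
; R, T and E each possess a character by its index in GetAllActorsOfClass, lighting its Flame component and turning off the other two.
; F possesses the first Flame actor and activates its particles, only when the level database's Pp1Pressed flag is set.
; The level database reference is looked up again every Tick.
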(event `self.ReceiveTick`
  (params (DeltaSeconds :type "Float (single-precision)"))
  (bind _outactors (`GameplayStatics.GetAllActorsOfClass` "/Game/Blueprints/LevelDatabaseActor.LevelDatabaseActor_C"))
  (set `self.levelDataBase` (`|GetArrayItem` _outactors)))

(event `Key|E`
  (params (Key :type "Key Structure"))
  (:`Pressed`
    (bind _outactors (`GameplayStatics.GetAllActorsOfClass` "/Game/SideScrollerBP/Blueprints/SideScrollerCharacter.SideScrollerCharacter_C"))
    (bind _output (`|GetArrayItem` _outactors 2))
    (`self.Possess` _output)
    (`ActorComponent.SetActive` (`/Game/SideScrollerBP/Blueprints/SideScrollerCharacter.flame` _output) true false)
    (bind _outactors_2 (`GameplayStatics.GetAllActorsOfClass` "/Game/SideScrollerBP/Blueprints/SideScrollerCharacter.SideScrollerCharacter_C"))
    (`ActorComponent.SetActive` (`/Game/SideScrollerBP/Blueprints/SideScrollerCharacter.flame` (`|GetArrayItem` _outactors_2)) false false)
    (`ActorComponent.SetActive` (`/Game/SideScrollerBP/Blueprints/SideScrollerCharacter.flame` (`|GetArrayItem` _outactors_2 1)) false false)))

(event `Key|T`
  (params (Key :type "Key Structure"))
  (:`Pressed`
    (bind _outactors (`GameplayStatics.GetAllActorsOfClass` "/Game/SideScrollerBP/Blueprints/SideScrollerCharacter.SideScrollerCharacter_C"))
    (bind _output (`|GetArrayItem` _outactors 1))
    (`self.Possess` _output)
    (`ActorComponent.SetActive` (`/Game/SideScrollerBP/Blueprints/SideScrollerCharacter.flame` _output) true false)
    (bind _outactors_2 (`GameplayStatics.GetAllActorsOfClass` "/Game/SideScrollerBP/Blueprints/SideScrollerCharacter.SideScrollerCharacter_C"))
    (`ActorComponent.SetActive` (`/Game/SideScrollerBP/Blueprints/SideScrollerCharacter.flame` (`|GetArrayItem` _outactors_2)) false false)
    (`ActorComponent.SetActive` (`/Game/SideScrollerBP/Blueprints/SideScrollerCharacter.flame` (`|GetArrayItem` _outactors_2 2)) false false)))

(event `Key|R`
  (params (Key :type "Key Structure"))
  (:`Pressed`
    (bind _outactors (`GameplayStatics.GetAllActorsOfClass` "/Game/SideScrollerBP/Blueprints/SideScrollerCharacter.SideScrollerCharacter_C"))
    (bind _output (`|GetArrayItem` _outactors))
    (`self.Possess` _output)
    (`ActorComponent.SetActive` (`/Game/SideScrollerBP/Blueprints/SideScrollerCharacter.flame` _output) true false)
    (bind _outactors_2 (`GameplayStatics.GetAllActorsOfClass` "/Game/SideScrollerBP/Blueprints/SideScrollerCharacter.SideScrollerCharacter_C"))
    (`ActorComponent.SetActive` (`/Game/SideScrollerBP/Blueprints/SideScrollerCharacter.flame` (`|GetArrayItem` _outactors_2 1)) false false)
    (`ActorComponent.SetActive` (`/Game/SideScrollerBP/Blueprints/SideScrollerCharacter.flame` (`|GetArrayItem` _outactors_2 2)) false false)))

(event `Key|F`
  (params (Key :type "Key Structure"))
  (:`Pressed`
    (if (`/Game/Blueprints/LevelDatabaseActor.pp1Pressed` (`self.levelDataBase`))
      (bind _outactors (`GameplayStatics.GetAllActorsOfClass` "/Game/SideScrollerBP/Blueprints/flame.flame_C"))
      (bind _output (`|GetArrayItem` _outactors))
      (`self.Possess` _output)
      (`ActorComponent.SetActive` (`/Game/SideScrollerBP/Blueprints/flame.ParticleSystem` _output) true false))))

(fn `UserConstructionScript`)