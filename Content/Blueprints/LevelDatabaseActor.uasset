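; Level state actor that holds three "Pp" pressed flags and the win condition for the level.
; On BeginPlay it caches the first AtmosphericFog actor found in the world.
; Tick polls the flags, which nothing in this graph sets; while all three are true it sets Won, prints "Gagné" and zeroes the fog's default brightness, repeating every frame with no one-shot guard.
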(event `self.ReceiveBeginPlay`
  (bind _outactors (`GameplayStatics.GetAllActorsOfClass` "/Script/Engine.AtmosphericFog"))
  (set `self.atmosphericFog` (`|GetArrayItem` _outactors)))

(event `self.ReceiveTick`
  (params (DeltaSeconds :type "Float (single-precision)"))
  (if (and (`self.pp1Pressed`) (`self.pp2Pressed`) (`self.pp3Pressed`))
    (set `self.won` true)
    (`KismetSystemLibrary.PrintString` "Gagné")
    (`AtmosphericFogComponent.SetDefaultBrightness` (`AtmosphericFog.AtmosphericFogComponent` (`self.atmosphericFog`)) 0.0)))

(fn `UserConstructionScript`)